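; BP_AI is a wandering test character that registers its movement with the Enhanced Tick System.
; On BeginPlay it starts a loop that sends its AI controller to random reachable points within a radius, pausing briefly after each move finishes.
; It also registers all CharacterMovementComponents with the Enhanced Tick System using the parallel flag, so their ticking can run in parallel.
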(event Custom|MoveLoop
  (bind _asaicontroller (Utilities|Casting|CastToAIController (Pawn|GetController)))
  (AI|AIMoveTo _asaicontroller (.RandomLocation (AI|Navigation|GetRandomReachablePointinRadius (Transformation|GetActorLocation) 1.5e+03 0 0)) 0 -1.0 "Default" "Default" true true
    (:OnMoveFinished
      (Utilities|FlowControl|Delay 0.2)
      (CallFunction|MoveLoop))))

(event EventBeginPlay
  (CallFunction|MoveLoop)
  (Class|EnhancedTickSystem|RegisterAllComponentsOfType (Subsystems|GetEnhancedTickSystem) "/Script/Engine.CharacterMovementComponent" "UseParallel") ; 3 ms
)

(fn ConstructionScript)