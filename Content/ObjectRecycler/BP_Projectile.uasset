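; Pooled projectile actor that deals point damage on hit and is recycled through an object pool manager instead of being destroyed.
; Pool events toggle visibility, collision and the active flag, with a request payload supplying requester, spawn transform and damage.
; A lifespan timer starts on valid spawn and clears on return.
; Hits damage actors other than itself or the requester, then return it to the pool.
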(event OnComponentHit(ProjectileMesh)
  (params (HitComponent :type Primitive%20Component%20Object%20Reference) (OtherActor :type Actor%20Object%20Reference) (OtherComp :type Primitive%20Component%20Object%20Reference) (NormalImpulse :type Vector :default "0, 0, 0") (Hit :type Hit%20Result%20Structure%20%28by%20ref%29))
  ;[0.15 0.15 0.15 0.5] Hit processing happens here
  (Variables|Default|SetOther%20Actor OtherActor)
  (Variables|Default|SetHit Hit)
  (Utilities|FlowControl|Sequence
    (:then_0
      (if (Math|Boolean|ANDBoolean (!= (Variables|Default|GetOther%20Actor) self) (Utilities|IsValid (Variables|Default|GetOther%20Actor)) (!= (Variables|Default|GetOther%20Actor) (Variables|Default|GetRequesting%20Actor)) (Variables|Default|GetbIsActive))
        (Game|Damage|ApplyPointDamage (Variables|Default|GetOther%20Actor) (Variables|ProjectileSettings|GetDamage) (.ImpactPoint (Collision|BreakHitResult (Variables|Default|GetHit))) (Variables|Default|GetHit))))
    (:then_1
      (CallFunction|ReturntoPool) ; Return to pool
    )))

(event EventObjectRequestedforUsage
  (params (Payload :type Object%20Pool%20Payload%20Structure))
  (bind (_requestingactor _spawnlocation _spawnrotation _floatparameters) (Utilities|Struct|BreakObjectPoolPayload Payload))
  (bind (_value _returnvalue) (Utilities|Map|Find _floatparameters "Damage"))
  ;[0.15 0.15 0.15 0.5] Called when the projectile is retrieved from the pool (like BeginPlay)
  (Rendering|SetActorHiddenInGame false)
  (Variables|Default|SetRequesting%20Actor _requestingactor)
  (Collision|SetActorEnableCollision true)
  (Variables|Default|SetbIsActive true)
  (if (not (Math|Vector|VectorIsZero _spawnlocation))
    (bind _returnvalue_2 (Utilities|Time|SetTimerbyEvent (EventDispatchers|CreateEvent :!event ReturntoPool) (Variables|ProjectileSettings|GetPoolableLifeSpan)))
    (Variables|Default|SetLifeSpanTimerHandle _returnvalue_2)
    (Transformation|SetActorLocation _spawnlocation false false)
    (if (not (Utilities|Operators|NotEqual(!=) :A _spawnrotation))
      (Transformation|SetActorRotation _spawnrotation)
      (if _returnvalue
        (Variables|ProjectileSettings|SetDamage _value)))))

(event EventAddedtoPool
  (params (Payload :type Object%20Pool%20Payload%20Structure))
  ;[0.15 0.15 0.15 0.5] Called when the projectile is first added to the pool
  (Rendering|SetActorHiddenInGame true)
  (Collision|SetActorEnableCollision false)
  (Components|Movement|StopMovementImmediately (Variables|Default|GetProjectileMovement))
  (Variables|Default|SetbIsActive false)
  (Utilities|Time|ClearandInvalidateTimerbyHandle (Variables|Default|GetLifeSpanTimerHandle)))

(event EventRemovedfromPool
  (params (Payload :type Object%20Pool%20Payload%20Structure))
  ;[0.15 0.15 0.15 0.5] Called when the projectile is permanently removed from the pool
)

(event EventReturnedtoPool
  (params (Payload :type Object%20Pool%20Payload%20Structure))
  ;[0.15 0.15 0.15 0.5] Called when the projectile is returned to the pool
  (Rendering|SetActorHiddenInGame true)
  (Collision|SetActorEnableCollision false)
  (Components|Movement|StopMovementImmediately (Variables|Default|GetProjectileMovement))
  (Variables|Default|SetbIsActive false)
  (Utilities|Time|ClearandInvalidateTimerbyHandle (Variables|Default|GetLifeSpanTimerHandle)))

(fn ConstructionScript
  (bind _projectilemesh (Variables|Default|GetProjectileMesh))
  (bind _projectilemovement (Variables|Default|GetProjectileMovement))
  (Physics|SetSimulatePhysics _projectilemesh true)
  (Physics|SetEnableGravity _projectilemesh false)
  (Class|PrimitiveComponent|SetNotifyRigidBodyCollision _projectilemesh true)
  (Components|Movement|SetUpdatedComponent _projectilemovement _projectilemesh)
  (Variables|/Script/Engine.ProjectileMovementComponent|SetInitialSpeed _projectilemovement (Variables|ProjectileSettings|GetInitial%20Speed))
  (Variables|/Script/Engine.ProjectileMovementComponent|SetMaxSpeed _projectilemovement (Variables|ProjectileSettings|GetMax%20Speed))
  (Variables|/Script/Engine.ProjectileMovementComponent|SetbRotationFollowsVelocity _projectilemovement true)
  (Variables|/Script/Engine.ProjectileMovementComponent|SetProjectileGravityScale _projectilemovement 0.0))

(fn ReturntoPool
  (if (Variables|Default|GetbIsActive)
    (Class|ObjectPoolManager|ReturnObjecttoPool (Subsystems|GetObjectPoolManager) self (LocalVariables|GetPayload))
    (else
      (return))))

(fn CanbeRecycled
  (return (not (Variables|Default|GetbIsActive))))